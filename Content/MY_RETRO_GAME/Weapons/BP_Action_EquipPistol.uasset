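; BP_Action_EquipPistol is a scripted action that gives the player a pistol.
; Its RunScript function finds the WeaponManagerComponent on player character 0 and calls EquipWeaponSmart with BP_Pistol for the first slot.
; Red Russian debug messages report the script start and the weapon handout.
; The event graph holds only disabled default nodes, so all logic sits in RunScript.
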(event EventBeginPlay
  (|CallParentFunction) ; This node is disabled and will not be called.\nDrag off pins to build functionality.
)

(event Collision|EventActorBeginOverlap
  (params (OtherActor :type Actor%20Object%20Reference))
  (|CallParentFunction OtherActor) ; This node is disabled and will not be called.\nDrag off pins to build functionality.
)

(event EventTick
  (params (DeltaSeconds :type Float%20%28single-precision%29))
  (|CallParentFunction DeltaSeconds) ; This node is disabled and will not be called.\nDrag off pins to build functionality.
)

(fn ConstructionScript
  (|CallParentFunction))

(fn RunScript
  (Development|PrintString "СКРИПТ ЗАПУЩЕН" true true "(R=1.000000,G=0.015196,B=0.000000,A=1.000000)")
  (Class|WeaponManagerComponent|EquipWeaponSmart (Actor|GetComponentbyClass (Game|GetPlayerCharacter 0) "/Script/RetroGame.WeaponManagerComponent") "/Game/MY_RETRO_GAME/Weapons/BP_Pistol.BP_Pistol_C")
  (Development|PrintString "ОРУЖИЕ ВЫДАНО" true true "(R=1.000000,G=0.013828,B=0.000000,A=1.000000)"))