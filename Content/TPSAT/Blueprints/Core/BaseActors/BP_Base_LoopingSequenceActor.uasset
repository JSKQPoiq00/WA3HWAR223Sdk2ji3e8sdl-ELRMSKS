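; Base interactable actor that lets the player sit down for a looping cinematic, with optional music, until they press Back.
; Left-button interaction hides the pawn and widgets, holds interaction tracing, then chains intro and looping Level Sequences through OnFinished.
; Leaving fades out music and plays an end sequence before restoring pawn, input and widgets.
; Top-button interaction plays data-table dialogue with optional camera focus.
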(event Custom|SitDown
  ;[0 0.7379 1] Main sequence mechanics
  ;;[1 1 1] Disable input, hide widgets, stop interaction trace
  (Variables|/Game/TPSAT/Blueprints/Core/BP_StoryAdv_GameController.BP_StoryAdv_GameController_C|SetHoldTrace (Variables|Default|GetGameControllerInstance) true)
  (bind _hiddenwidgets (CallFunction|HideActiveWidgets))
  (Variables|Default|SetHiddenWidgets _hiddenwidgets)
  (Rendering|SetActorHiddenInGame (Game|Player|GetPlayerPawn 0) true)
  (Input|DisableInput (Variables|Default|GetGameControllerInstance) (Game|GetPlayerController 0))
  ;;[1 1 1] Fade in music, play intro sequence and start playing the loop afterwards
  (CallFunction|PlayMusic)
  (bind _outactor (Sequencer|Player|CreateLevelSequencePlayer (Variables|Sequences|GetStartSequence)))
  (bind _output_get (Variables|Default|SetCurrentSequenceActor _outactor))
  (Sequencer|Player|Play (Variables|/Script/LevelSequence.LevelSequenceActor|GetSequencePlayer _output_get) :!class /Script/MovieScene.MovieSceneSequencePlayer)
  (EventDispatchers|AssignOnFinished (Variables|/Script/LevelSequence.LevelSequenceActor|GetSequencePlayer _output_get) (delegate Custom|IntroFinished)))

(event Custom|IntroFinished
  (bind _gamecontrollerinstance (Variables|Default|GetGameControllerInstance))
  (bind _messagewidget (Variables|/Game/TPSAT/Blueprints/Core/BP_StoryAdv_GameController.BP_StoryAdv_GameController_C|GetMessageWidget _gamecontrollerinstance))
  ;[0 0.7379 1] Main sequence mechanics
  ;;[1 1 1] Fade in music, play intro sequence and start playing the loop afterwards
  (Actor|DestroyActor (Variables|Default|GetCurrentSequenceActor))
  (bind _outactor (Sequencer|Player|CreateLevelSequencePlayer (Variables|Sequences|GetLoopSequence)))
  (bind _output_get (Variables|Default|SetCurrentSequenceActor _outactor))
  (Class|MovieSceneSequencePlayer|PlayLooping (Variables|/Script/LevelSequence.LevelSequenceActor|GetSequencePlayer _output_get) -1)
  (Utilities|FlowControl|Delay 1.0)
  (Default|FadeinBottomRightBoxRight (Variables|/Game/TPSAT/Blueprints/Core/BP_StoryAdv_GameController.BP_StoryAdv_GameController_C|GetMessageWidget (Variables|Default|GetGameControllerInstance)) "Leave")
  (Input|EnableInput (Game|GetPlayerController 0))
  (Utilities|FlowControl|Delay 4.0)
  (UserInterface|Animation|PlayAnimation _messagewidget (Variables|/Game/TPSAT/UserInterface/WBP_MessageHUD.WBP_MessageHUD_C|GetFadeBottomRightBox_Right _messagewidget) 0.0 1 "Reverse" 1.0 false))

(event Custom|EndSequenceFinished
  ;[0 0.7379 1] Main sequence mechanics
  ;;[1 1 1] Stop loop sequence, play end sequence and switch back to game
  (Actor|DestroyActor (Variables|Default|GetCurrentSequenceActor))
  (Utilities|FlowControl|Delay 0.2)
  (Rendering|SetActorHiddenInGame (Game|Player|GetPlayerPawn 0) false)
  (Input|EnableInput (Game|Player|GetPlayerPawn 0) (Game|GetPlayerController 0))
  (CallFunction|ShowHiddenWidgets (Variables|Default|GetHiddenWidgets))
  (Variables|/Game/TPSAT/Blueprints/Core/BP_StoryAdv_GameController.BP_StoryAdv_GameController_C|SetHoldTrace (Variables|Default|GetGameControllerInstance) false))

(event Custom|PlayMusic
  ;[0 0.7379 1] Main sequence mechanics
  ;;[1 1 1] Play music
  (Utilities|IsValid (Variables|MusicSetup|GetSong)
    (:Is%20Valid
      (Utilities|FlowControl|Delay (Variables|MusicSetup|GetMusicStartDelay))
      (bind _returnvalue (Audio|SpawnSound2D (Variables|MusicSetup|GetSong) 1.0 1.0 0.0 0))
      (bind _output_get (Variables|Default|SetMusicPlayer _returnvalue))
      (Audio|Components|Audio|FadeIn (Variables|Default|GetMusicPlayer) (Variables|MusicSetup|GetFadeInDuration) 1.0 0.0 "Linear" :!class /Script/Engine.AudioComponent))))

(event Custom|Leave
  ;[0 0.7379 1] Main sequence mechanics
  ;;[1 1 1] Stop loop sequence, play end sequence and switch back to game
  (Input|DisableInput (Game|GetPlayerController 0))
  (Widget|SetVisibility (Variables|/Game/TPSAT/UserInterface/WBP_MessageHUD.WBP_MessageHUD_C|GetBottomRightInfoBox_Right (Variables|/Game/TPSAT/Blueprints/Core/BP_StoryAdv_GameController.BP_StoryAdv_GameController_C|GetMessageWidget (Variables|Default|GetGameControllerInstance))) "Collapsed")
  (Utilities|FlowControl|Delay 0.5)
  (Class|MovieSceneSequencePlayer|GotoEndandStop (Variables|/Script/LevelSequence.LevelSequenceActor|GetSequencePlayer (Variables|Default|GetCurrentSequenceActor)))
  (Actor|DestroyActor (Variables|Default|GetCurrentSequenceActor))
  (bind _musicplayer (Variables|Default|GetMusicPlayer)
    (:then
      (Audio|Components|Audio|FadeOut _musicplayer (Variables|MusicSetup|GetFadeOutDuration) 0.0 "Linear" :!class /Script/Engine.AudioComponent))
    (:else
      _))
  (bind _outactor (Sequencer|Player|CreateLevelSequencePlayer (Variables|Sequences|GetEndSequence)))
  (Variables|Default|SetCurrentSequenceActor _outactor)
  (Sequencer|Player|Play (Variables|/Script/LevelSequence.LevelSequenceActor|GetSequencePlayer _outactor) :!class /Script/MovieScene.MovieSceneSequencePlayer)
  (EventDispatchers|AssignOnFinished (Variables|/Script/LevelSequence.LevelSequenceActor|GetSequencePlayer _outactor) (delegate Custom|EndSequenceFinished)))

(event EventLeftButtonInteraction
  ;[0 0.7379 1] Input
  ;;[1 1 1] Bottom button interaction
  (CallFunction|SitDown))

(event EventTopButtonInteraction
  ;[0 0.7379 1] Input
  ;;[1 1 1] Inspect interaction
  (Utilities|FlowControl|Sequence
    (:then_0
      (bind (_dialogue_waves _subtitles _validdata) (CallFunction|GetDialogueDatafromTable (Variables|Default|GetDialogueRow)))
      (if _validdata
        (Default|PlayPlayerDialogue (Variables|Default|GetGameControllerInstance) _dialogue_waves _subtitles)))
    (:then_1
      (if (Variables|Default|GetUseCameraFocus)
        (CallFunction|CameraFocus)))))

(event Input|ActionEvents|InputActionBack
  (params (Key :type Key%20Structure :default "None"))
  ;[0 0.7379 1] Input
  ;;[1 1 1] Leave input
  (:Pressed
    (CallFunction|Leave)))

(fn ConstructionScript
  (|CallParentFunction))