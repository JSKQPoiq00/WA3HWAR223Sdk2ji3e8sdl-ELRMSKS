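; BP_UseAction_Pistol is a use-action actor that equips the player with a pistol.
; Its RunScript function casts the first player character to BP_StoryAdv_Character and looks up its WeaponManagerComponent.
; If that component is valid, it calls EquipWeapon with BP_Pistol.
; The event graph holds only disabled default events, so all behavior lives in RunScript.
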(event EventBeginPlay
  (|CallParentFunction) ; This node is disabled and will not be called.\nDrag off pins to build functionality.
)

(event Collision|EventActorBeginOverlap
  (params (OtherActor :type Actor%20Object%20Reference))
  (|CallParentFunction OtherActor) ; This node is disabled and will not be called.\nDrag off pins to build functionality.
)

(event EventTick
  (params (DeltaSeconds :type Float%20%28single-precision%29))
  (|CallParentFunction DeltaSeconds) ; This node is disabled and will not be called.\nDrag off pins to build functionality.
)

(fn ConstructionScript
  (|CallParentFunction))

(fn RunScript
  (bind _asbp_story_adv_character (Utilities|Casting|CastToBP_StoryAdv_Character (Game|GetPlayerCharacter 0)))
  (if (Utilities|IsValid (Actor|GetComponentbyClass _asbp_story_adv_character "/Script/RetroGame.WeaponManagerComponent"))
    (Class|WeaponManagerComponent|EquipWeapon (Actor|GetComponentbyClass _asbp_story_adv_character "/Script/RetroGame.WeaponManagerComponent") "/Game/MY_RETRO_GAME/Weapons/BP_Pistol.BP_Pistol_C")))