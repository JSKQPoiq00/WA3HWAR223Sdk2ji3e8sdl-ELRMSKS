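; BP_UseAction_Equip is an item use action that equips a weapon on the player character.
; RunScript checks that the weapon class in ItemProperties is valid and casts the first player character to BP_StoryAdv_Character.
; It then passes that class to EquipWeapon on the character's WeaponManagerComponent.
; The event graph holds only disabled placeholder events.
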(event EventBeginPlay
  (|CallParentFunction) ; This node is disabled and will not be called.\nDrag off pins to build functionality.
)

(event Collision|EventActorBeginOverlap
  (params (OtherActor :type Actor%20Object%20Reference))
  (|CallParentFunction OtherActor) ; This node is disabled and will not be called.\nDrag off pins to build functionality.
)

(event EventTick
  (params (DeltaSeconds :type Float%20%28single-precision%29))
  (|CallParentFunction DeltaSeconds) ; This node is disabled and will not be called.\nDrag off pins to build functionality.
)

(fn ConstructionScript
  (|CallParentFunction))

(fn RunScript
  (bind _itemproperties (Variables|Default|GetItemProperties))
  (bind _weaponclass (Utilities|Struct|BreakBP_InventoryItem _itemproperties))
  (if (Utilities|IsValidClass _weaponclass)
    (bind _asbp_story_adv_character (Utilities|Casting|CastToBP_StoryAdv_Character (Game|GetPlayerCharacter 0)))
    (Class|WeaponManagerComponent|EquipWeapon (Actor|GetComponentbyClass _asbp_story_adv_character "/Script/RetroGame.WeaponManagerComponent") _weaponclass)))