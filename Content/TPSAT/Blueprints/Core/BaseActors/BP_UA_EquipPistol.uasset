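; BP_UA_EquipPistol is a scripted action actor that equips the player with a pistol.
; Its RunScript override calls the parent, then casts player character 0 to BP_StoryAdv_Character, stopping if the cast fails.
; It spawns a BP_Weapon_Pistol, attaches it to the mesh's RightHand socket and stores it as CurrentWeapon, without handling any previously held weapon.
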(event EventBeginPlay
  (|CallParentFunction) ; This node is disabled and will not be called.\nDrag off pins to build functionality.
)

(event Collision|EventActorBeginOverlap
  (params (OtherActor :type Actor%20Object%20Reference))
  (|CallParentFunction OtherActor) ; This node is disabled and will not be called.\nDrag off pins to build functionality.
)

(event EventTick
  (params (DeltaSeconds :type Float%20%28single-precision%29))
  (|CallParentFunction DeltaSeconds) ; This node is disabled and will not be called.\nDrag off pins to build functionality.
)

(fn ConstructionScript
  (|CallParentFunction))

(fn RunScript
  (|CallParentFunction)
  (bind _asbp_story_adv_character (Utilities|Casting|CastToBP_StoryAdv_Character (Game|GetPlayerCharacter 0)))
  (bind _returnvalue (Game|SpawnActorfromClass "/Game/MY_RETRO_GAME/Weapons/BP_Weapon_Pistol.BP_Weapon_Pistol_C" (Math|Transform|MakeTransform "0, 0, 0" "0, 0, 0" "1.000000,1.000000,1.000000") "Undefined" "MultiplyWithRoot" 0 0))
  (Transformation|AttachComponentToComponent _returnvalue (Variables|/Script/Engine.Character|GetMesh _asbp_story_adv_character) "RightHand" "SnapToTarget" "SnapToTarget" "KeepRelative" true)
  (Variables|/Game/TPSAT/Blueprints/Character/BP_StoryAdv_Character.BP_StoryAdv_Character_C|SetCurrentWeapon _asbp_story_adv_character _returnvalue))